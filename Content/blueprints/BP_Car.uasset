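; BP_Car is a moving hazard that restarts the current level when BP_Player overlaps it.
; Each tick it moves along its root's forward vector at Speed, without sweeping.
; Once it is farther than Distance from StartPosition it teleports back there, forming an endless loop.
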(event `self.ReceiveActorBeginOverlap`
  (params (OtherActor :type "Actor Object Reference"))
  (cast `/Game/blueprints/BP_Player` OtherActor)
  (bind _returnvalue (`GameplayStatics.GetCurrentLevelName` true))
  (`GameplayStatics.OpenLevel` (`KismetStringLibrary.Conv_StringToName` _returnvalue)))

(event `self.ReceiveTick`
  (params (DeltaSeconds :type "Float (single-precision)"))
  (`self.K2_AddActorWorldOffset` (* (`SceneComponent.GetForwardVector` (`self.DefaultSceneRoot`)) (* DeltaSeconds (`self.Speed`))))
  (if (> (`KismetMathLibrary.Vector_Distance` (`self.K2_GetActorLocation`) (`self.StartPosition`)) (`self.Distance`))
    (`self.K2_SetActorLocation` (`self.StartPosition`))))

(fn `UserConstructionScript`)