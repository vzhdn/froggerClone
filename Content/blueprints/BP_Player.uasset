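; Player pawn that moves in fixed grid steps along four directions and keeps a score.
; BeginPlay resets it to the world origin, adds the Enhanced Input mapping context and creates the game UI.
; Input actions call TryMove, which shifts TargetPos and locks further moves behind a short timer, while Tick drives the root component toward that target with MoveComponentTo.
; AddScore accumulates points and pushes the total to the UI.
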(event `self.ReceiveBeginPlay`
  (`self.K2_SetActorLocation` (0.0 0.0 0.0))
  (set `self.TargetPos` (`self.K2_GetActorLocation`))
  (bind _asplayer_controller (cast `PlayerController` (`self.GetController`)))
  (bind _returnvalue (pcsubsystem `EnhancedInputLocalPlayerSubsystem` _asplayer_controller))
  (`/Engine/EditorBlueprintResources/StandardMacros.IsValid` _returnvalue
    (:`Is Valid`
      (`EnhancedInputSubsystemInterface.AddMappingContext` _returnvalue "/Game/input/IMC_Default.IMC_Default" 0 (struct))
      (bind _returnvalue_2 (`|CreateWidget` "/Game/blueprints/GameUI.GameUI_C" (`GameplayStatics.GetPlayerController` 0)))
      (`UserWidget.AddToViewport` _returnvalue_2 0)
      (set `self.GameUI` _returnvalue_2))))

(event `EnhancedInput|/Game/input/IA_MoveForward`
  (params (ActionValue :type Boolean) (ElapsedSeconds :type "Float (double-precision)") (TriggeredSeconds :type "Float (double-precision)") (InputAction :type "InputAction Object Reference" :default "/Game/input/IA_MoveForward.IA_MoveForward"))
  (:`Triggered`
    (`self.TryMove` (100.0 0.0 0.0))))

(event `self.ReceiveTick`
  (params (DeltaSeconds :type "Float (single-precision)"))
  (`KismetSystemLibrary.MoveComponentTo` (`self.DefaultSceneRoot`) (`self.TargetPos`)))

(event `EnhancedInput|/Game/input/IA_MoveLeft`
  (params (ActionValue :type Boolean) (ElapsedSeconds :type "Float (double-precision)") (TriggeredSeconds :type "Float (double-precision)") (InputAction :type "InputAction Object Reference" :default "/Game/input/IA_MoveLeft.IA_MoveLeft"))
  (:`Triggered`
    (`self.TryMove` (0.0 -100.0 0.0))))

(event `EnhancedInput|/Game/input/IA_MoveRight`
  (params (ActionValue :type Boolean) (ElapsedSeconds :type "Float (double-precision)") (TriggeredSeconds :type "Float (double-precision)") (InputAction :type "InputAction Object Reference" :default "/Game/input/IA_MoveRight.IA_MoveRight"))
  (:`Triggered`
    (`self.TryMove` (0.0 100.0 0.0))))

(event `EnhancedInput|/Game/input/IA_MoveBackwards`
  (params (ActionValue :type Boolean) (ElapsedSeconds :type "Float (double-precision)") (TriggeredSeconds :type "Float (double-precision)") (InputAction :type "InputAction Object Reference" :default "/Game/input/IA_MoveBackwards.IA_MoveBackwards"))
  (:`Triggered`
    (`self.TryMove` (-100.0 0.0 0.0))))

(fn `AddScore`
  (params (ScoreToAdd :type Integer))
  (bind _output_get (set `self.Score` (+ ScoreToAdd (`self.Score`))))
  (`/Game/blueprints/GameUI.UpdateScore` (`self.GameUI`) _output_get))

(fn `EnableCanMove`
  (set `self.CanMove` true))

(fn `TryMove`
  (params (Direction :type "Vector Structure"))
  (if (`self.CanMove`)
    (set `self.TargetPos` (+ Direction (`self.TargetPos`)))
    (set `self.CanMove` false)
    (`KismetSystemLibrary.K2_SetTimer` null "EnableCanMove" 0.3)))

(fn `UserConstructionScript`)